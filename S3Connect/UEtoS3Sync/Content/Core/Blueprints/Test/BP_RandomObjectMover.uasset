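; Test actor that populates a square map area with randomly placed BP_AWS actors and keeps relocating them.
; On BeginPlay, FnCreateTargets spawns the actors at random positions and rotations, gives each a random SyncEverySeconds and stores them in Objects.
; Tick uses a DoOnce, reset on odd game seconds, to teleport one random entry every two seconds via FnRandomLocation.
; The debug print rolls its own random transform rather than showing the applied one.
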(event `self.ReceiveBeginPlay`
  (`self.fnCreateTargets` (28000.0 28000.0) 50))

(event `self.ReceiveTick`
  (params (DeltaSeconds :type "Float (single-precision)"))
  (bind _transform (`self.fnRandomLocation` (28000.0 28000.0)))
  (bind _objects (`self.Objects`))
  (if (== (mod (`KismetMathLibrary.FFloor` (`KismetSystemLibrary.GetGameTimeInSeconds`)) 2) 0)
    (`/Engine/EditorBlueprintResources/StandardMacros.DoOnce` false :!label _label
      (:`Completed`
        (`self.K2_SetActorTransform` (`|GetArrayItem` _objects (`KismetMathLibrary.RandomIntegerInRange` 0 (`KismetArrayLibrary.Array_Length` _objects))) _transform false false)
        (`KismetSystemLibrary.PrintString` (`KismetStringLibrary.Conv_TransformToString` _transform))))
    (else
      (goto _label :!via `Reset`))))

(fn `fnCreateTargets`
  (params (MapSize :type "Vector2D Structure") (Count :type Integer))
  (bind (_x _y) (`KismetMathLibrary.BreakVector2D` MapSize))
  (bind _returnvalue (/ _y 2.0))
  (bind _returnvalue_2 (/ _x 2.0))
  (for _ (range (+ Count 1))
    (bind _returnvalue_3 (`|SpawnActorFromClass` "/Game/Core/Blueprints/Test/BP_AWS.BP_AWS_C" (`KismetMathLibrary.MakeTransform` (`KismetMathLibrary.MakeVector` (`KismetMathLibrary.RandomFloatInRange` (* -1 _returnvalue_2) _returnvalue_2) (`KismetMathLibrary.RandomFloatInRange` (* -1 _returnvalue) _returnvalue) 50.0) (`KismetMathLibrary.RandomRotator` true)) "Undefined" "OverrideRootScale" null null))
    (set `/Game/Core/Blueprints/Test/BP_AWS.SyncEverySeconds` (`KismetMathLibrary.RandomIntegerInRange` 5 15) _returnvalue_3)
    (`KismetArrayLibrary.Array_Add` (`self.Objects`) _returnvalue_3)))

(fn `fnRandomLocation`
  (params (MapSize :type "Vector2D Structure"))
  (returns (Transform :type "Transform Structure"))
  (bind (_x _y) (`KismetMathLibrary.BreakVector2D` MapSize))
  (bind _returnvalue (/ _y 2.0))
  (bind _returnvalue_2 (/ _x 2.0))
  (return (`KismetMathLibrary.MakeTransform` (`KismetMathLibrary.MakeVector` (`KismetMathLibrary.RandomFloatInRange` (* -1 _returnvalue_2) _returnvalue_2) (`KismetMathLibrary.RandomFloatInRange` (* -1 _returnvalue) _returnvalue) 50.0))))

(fn `UserConstructionScript`)