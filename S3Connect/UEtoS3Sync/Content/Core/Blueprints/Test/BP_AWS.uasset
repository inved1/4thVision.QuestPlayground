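; Test actor that periodically POSTs its transform as JSON to a configurable URL, using one reusable VaRest-style request created on BeginPlay.
; Tick uses game-time modulo and a DoOnce to fire once per interval, sending only when the request is idle, succeeded or failed.
; Each payload carries a fresh GUID, Unix time and transform; responses are printed.
; FnLogEveryXSeconds and a second send chain are unused duplicates.
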(event `evtRequestComplete`
  (params (Request :type "VaRestRequestJSON Object Reference"))
  (bind _returnvalue (`VaRestRequestJSON.GetResponseObject` Request))
  (`KismetSystemLibrary.PrintString` (`VaRestJsonObject.EncodeJson` _returnvalue)))

(event `evtRequestFailed`
  (params (Request :type "VaRestRequestJSON Object Reference"))
  (bind _returnvalue (`VaRestRequestJSON.GetResponseObject` Request))
  (`KismetSystemLibrary.PrintString` (`VaRestJsonObject.EncodeJson` _returnvalue)))

(event `self.ReceiveBeginPlay`
  (bind _tmprequest (`self.tmpRequest`))
  (`self.fnInitRequest`)
  (`|ExecutionSequence`
    (:`then_0`
      (add `VaRestRequestJSON.OnRequestComplete` _tmprequest (delegate `evtRequestComplete`)))
    (:`then_1`
      (add `VaRestRequestJSON.OnRequestFail` _tmprequest (delegate `evtRequestFailed`)))))

(event `self.ReceiveTick`
  (params (DeltaSeconds :type "Float (single-precision)"))
  (bind _tmprequest (`self.tmpRequest`))
  (if (== (mod (`KismetMathLibrary.FFloor` (`KismetSystemLibrary.GetGameTimeInSeconds`)) (`self.SyncEverySeconds`)) 0)
    (`/Engine/EditorBlueprintResources/StandardMacros.DoOnce` false :!label _label
      (:`Completed`
        (bind _returnvalue (`VaRestRequestJSON.GetStatus` (`self.tmpRequest`)))
        (switch `ERequestStatus` _returnvalue
          (:`NotStarted`
            _)
          (:`Failed`
            _)
          (:`Failed_ConnectionError`
            _)
          (:`Succeeded`
            _))
        (`|ExecutionSequence`
          (:`then_1`
            (`|ExecutionSequence`
              (:`then_0`
                (bind _returnvalue_2 (`VaRestRequestJSON.GetRequestObject` (`self.tmpRequest`)))
                (`VaRestJsonObject.SetField` _returnvalue_2 "GUID" (`VaRestJsonValue.ConstructJsonValueString` (`KismetGuidLibrary.Conv_GuidToString` (`KismetGuidLibrary.NewGuid`)))))
              (:`then_1`
                (bind _returnvalue_3 (`VaRestRequestJSON.GetRequestObject` (`self.tmpRequest`)))
                (`VaRestJsonObject.SetField` _returnvalue_3 "TM" (`VaRestJsonValue.ConstructJsonValueNumber` (`KismetMathLibrary.GetTotalSeconds` (- (`KismetMathLibrary.Now`) (`KismetMathLibrary.MakeDateTime` 1 1 1970))))))
              (:`then_2`
                (bind _returnvalue_4 (`VaRestRequestJSON.GetRequestObject` (`self.tmpRequest`)))
                (`VaRestJsonObject.SetField` _returnvalue_4 "Transform" (`VaRestJsonValue.ConstructJsonValueString` (`KismetStringLibrary.Conv_TransformToString` (`self.GetTransform`)))))))
          (:`then_2`
            (`VaRestRequestJSON.SetURL` _tmprequest (`self.FRequestURL`)))
          (:`then_3`
            (`VaRestRequestJSON.ExecuteProcessRequest` _tmprequest)))))
    (else
      (goto _label :!via `Reset`))))

(fn `fnInitRequest`
  (set `self.tmpRequest` (`VaRestRequestJSON.ConstructRequestExt` "POST" "json"))
  (return))

(fn `fnLogEveryXSeconds`
  (params (XSecond :type Integer))
  (locals (bIsRunning :type Boolean))
  (bind _tmprequest (`self.tmpRequest`))
  (if (== (mod (`KismetMathLibrary.FFloor` (`KismetSystemLibrary.GetGameTimeInSeconds`)) XSecond) 0)
    (`/Engine/EditorBlueprintResources/StandardMacros.DoOnce` false :!label _label
      (:`Completed`
        (`|ExecutionSequence`
          (:`then_1`
            (`|ExecutionSequence`
              (:`then_0`
                (bind _returnvalue (`VaRestRequestJSON.GetRequestObject` (`self.tmpRequest`)))
                (`VaRestJsonObject.SetField` _returnvalue "GUID" (`VaRestJsonValue.ConstructJsonValueString` (`KismetGuidLibrary.Conv_GuidToString` (`KismetGuidLibrary.NewGuid`)))))
              (:`then_1`
                (bind _returnvalue_2 (`VaRestRequestJSON.GetRequestObject` (`self.tmpRequest`)))
                (`VaRestJsonObject.SetField` _returnvalue_2 "TM" (`VaRestJsonValue.ConstructJsonValueNumber` (`KismetMathLibrary.GetTotalSeconds` (- (`KismetMathLibrary.Now`) (`KismetMathLibrary.MakeDateTime` 1 1 1970))))))
              (:`then_2`
                (bind _returnvalue_3 (`VaRestRequestJSON.GetRequestObject` (`self.tmpRequest`)))
                (`VaRestJsonObject.SetField` _returnvalue_3 "Transform" (`VaRestJsonValue.ConstructJsonValueString` (`KismetStringLibrary.Conv_TransformToString` (`self.GetTransform`)))))))
          (:`then_2`
            (`VaRestRequestJSON.SetURL` _tmprequest (`self.FRequestURL`)))
          (:`then_3`
            (`VaRestRequestJSON.ExecuteProcessRequest` _tmprequest)))))
    (else
      (goto _label :!via `Reset`))))

(fn `UserConstructionScript`)